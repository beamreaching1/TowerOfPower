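; BP_LavaPlatform_2 is a platform that turns to lava and restarts the current level when the player touches it in that state.
; A hit from anything other than the player pawn switches its material to M_inferno after a short delay.
; A player hit reloads the level by name only if that material is already applied, so the material itself serves as the hazard flag.
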(event OnComponentHit(Platform)
  (params (HitComponent :type Primitive%20Component%20Object%20Reference) (OtherActor :type Actor%20Object%20Reference) (OtherComp :type Primitive%20Component%20Object%20Reference) (NormalImpulse :type Vector :default "0, 0, 0") (Hit :type Hit%20Result%20Structure%20%28by%20ref%29))
  (if (== OtherActor (Game|Player|GetPlayerPawn 0))
    (if (== (Rendering|Material|GetMaterial (Variables|Default|GetPlatform) 0) "/Game/NecrosUtilityMatPack/materials/misc/masters/m_inferno.m_inferno")
      (bind _returnvalue (Game|GetCurrentLevelName true))
      (Game|OpenLevel(byName) (Utilities|String|StringToName _returnvalue)))
    (else
      (Utilities|FlowControl|Delay 5.0)
      (Rendering|Material|SetMaterial (Variables|Default|GetPlatform) 0 "/Game/NecrosUtilityMatPack/materials/misc/masters/m_inferno.m_inferno"))))

(event EventBeginPlay)

(event EventTick
  (params (DeltaSeconds :type Float%20%28single-precision%29)))

(fn ConstructionScript)